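; Player controller that casts skills for the player character, either at a clicked location or along a direction.
; A location cast turns the character toward the point with zero pitch, then re-broadcasts as a direction cast.
; Direction casts spawn the skill row's Blueprint at the character, passing scale, damage and a fixed duration.
; GetSkillsWithInput returns Enhanced Input key names alongside skill rows looked up by enum name in the skill DataTable.
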(event Custom|evOnLocationClick_Event
  (params (aClickLocation :type Vector) (aSkillData :type Skill%20Data%20Row%20Structure%20%28by%20ref%29))
  (CallFunction|CastLocationSkill aClickLocation aSkillData))

(event Custom|evOnDirectionSkillCast_Event
  (params (aRotation :type Rotator) (aSkillData :type Skill%20Data%20Row%20Structure))
  (|CollapseGraph aRotation aSkillData))

(event EventBeginPlay
  (EventDispatchers|AssignEvonLocationClick (delegate Custom|evOnLocationClick_Event))
  (EventDispatchers|AssignEvonDirectionSkillCast (delegate Custom|evOnDirectionSkillCast_Event)))

(fn ConstructionScript)

(fn GetLooktoTarget
  (params (aLocation :type Vector))
  (bind _mpplayercharacter (Variables|Default|GetmpPlayerCharacter))
  (bind _returnvalue (Transformation|GetActorLocation _mpplayercharacter))
  (bind _returnvalue_2 (Math|Rotator|FindLookatRotation _returnvalue aLocation))
  (bind (_roll _pitch _yaw) (Math|Rotator|BreakRotator _returnvalue_2))
  (return (Math|Rotator|MakeRotator _roll 0.0 _yaw)))

(fn CastLocationSkill
  (params (InputPin :type Vector) (Inpuut%20Pin :type Skill%20Data%20Row%20Structure))
  (if true
    (bind _output_get (LocalVariables|SetRot (CallFunction|GetLooktoTarget InputPin)))
    (Transformation|SetActorRotation (Variables|Default|GetmpPlayerCharacter) _output_get)
    (Default|CallEvonDirectionSkillCast (LocalVariables|GetRot) Inpuut%20Pin)))

(fn GetSkillswithInput
  (bind _tskills (LocalVariables|GettSkills))
  (Utilities|FlowControl|Sequence
    (:then_0
      ;[1 1 1] Keypress
      (for _array_element (Variables|/Script/RPG_2024_PolGarriga.InputConfigData|GetmpInputSkills (Variables|Default|GetmpInputData))
        (bind _returnvalue (Class|EnhancedInputSubsystemInterface|QueryKeysMappedtoAction(Message) (PlayerController|LocalPlayerSubsystems|GetEnhancedInputLocalPlayerSubsystem) _array_element))
        (Utilities|Array|Add (LocalVariables|GettKeys) (Utilities|String|ToString(Text) (Class|KismetInputLibrary|KeyGetDisplayName (Utilities|Array|Get(acopy) _returnvalue) true)))))
    (:then_1
      ;[1 1 1 1 42] Skills
      (for _array_element_2 (Variables|Default|GetmSkills)
        (bind _returnvalue_2 (Utilities|GetDataTableRow (Variables|Default|GetmSkillDB) (Utilities|String|StringToName (Utilities|String|EnumtoString _array_element_2)))
          (:then
            (Utilities|Array|Add _tskills _returnvalue_2))
          (:RowNotFound
            (Utilities|Array|Add _tskills _returnvalue_2)))))
    (:then_2
      (return (LocalVariables|GettKeys) (LocalVariables|GettSkills)))))