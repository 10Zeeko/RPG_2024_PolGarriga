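; Enemy wave spawner Blueprint that adds a rune circle glow effect when an enemy spawns.
; On BeginPlay it binds to the EnemySpawned dispatcher, creates a dynamic material instance and passes it to the BP_Rune_Sphere_Circle_01 child actor.
; Each spawn event prints a debug string and restarts the Bright timeline, which drives the material's ColorPower parameter.
; The graph holds only this feedback, with no wave or spawning logic.
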(event Custom|EnemySpawned_Event
  (Development|PrintString "Spawned")
  (bind _bright (Timeline|Bright PlayFromStart)
    (:Update
      (Rendering|Material|SetScalarParameterValue (Variables|Default|GetDynamic) "ColorPower" _bright :!class /Script/Engine.MaterialInstanceDynamic))))

(event EventBeginPlay
  (EventDispatchers|AssignEnemySpawned (delegate Custom|EnemySpawned_Event))
  (bind _returnvalue (Rendering|Material|CreateDynamicMaterialInstance (Variables|Default|GetMaterial) "None" "None" :!class /Script/Engine.KismetMaterialLibrary))
  (Variables|Default|SetDynamic _returnvalue)
  (bind _asbp_rune_sphere_circle_01 (Utilities|Casting|CastToBP_Rune_Sphere_Circle_01 (Variables|/Script/Engine.ChildActorComponent|GetChildActor (Variables|Default|GetChildActor))))
  (Default|ChangeMaterial _asbp_rune_sphere_circle_01 (Variables|Default|GetDynamic)))

(fn ConstructionScript)